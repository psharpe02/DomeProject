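; Camera_2D is a cine camera rig for shots and image-sequence recording, with optional stereo.
; It can ride a spline, follow or look at targets, track static meshes entering its trigger sphere, or copy another actor's transform and CineCamera settings.
; Recording caps FPS, then pauses each frame for numbered HighResShot captures until the frame count is reached.
; Stereo creates extra players, spawns a Camera2D_R right-eye camera and applies an IPD offset.
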(event `self.ReceiveBeginPlay`
  (`|ExecutionSequence`
    (:`then_0`
      ;[1 1 1] Moving Camera>?
      (if (`self.StartCamera_Spline`)
        (`self.MovingCamera`)))
    (:`then_1`
      ;[1 0.473 1] Activate Camera . Update 1.12
      (if (`self.ActivateCamera?`)
        (`PlayerController.SetViewTargetWithBlend` (`GameplayStatics.GetPlayerController` 0) self 0.0 "VTBlend_Linear" 0.0 false)
        ;[0.5771 1 0.1143] Stereo 2D Activation. Update 1.13 Fix 2
        (if (`self.Stereo?`)
          (`self.Activation_Stereo2D`))))
    (:`then_2`
      (if (`self.Rec`)
        ;[0.3002 1 0.4822] Max FPS for Rec. Update 1.13
        (`KismetSystemLibrary.ExecuteConsoleCommand` (`KismetStringLibrary.Concat_StrStr` "t.MaxFPS " (`KismetStringLibrary.Conv_DoubleToString` (`self.Frame Rate Rec`))) null)
        (else
          ;[0.3728 1 0.3948] Max FPS for Editor. Update 1.13
          (`KismetSystemLibrary.ExecuteConsoleCommand` (`KismetStringLibrary.Concat_StrStr` "t.MaxFPS " (`KismetStringLibrary.Conv_DoubleToString` (`self.Max FPS for Editor`))) null))))))

(event `self.ReceiveTick`
  (params (DeltaSeconds :type "Float (single-precision)"))
  (bind _target_lookat (`self.Target_LookAT`))
  (bind _camera_arm (`self.Camera_arm`))
  (bind _target_follow (`self.Target_Follow`))
  (bind _cinecamera2d (`self.CineCamera2D`))
  (bind _current_shot (`self.Current Shot`))
  (`|ExecutionSequence`
    (:`then_0`
      ;[1 1 1] Look AT
      (`/Engine/EditorBlueprintResources/StandardMacros.IsValid` _target_lookat
        (:`Is Valid`
          (`self.LookAT`))))
    (:`then_1`
      ;[1 1 1] Follow
      (`/Engine/EditorBlueprintResources/StandardMacros.IsValid` _target_follow
        (:`Is Valid`
          (`self.Follow`)
          ;[1 1 1] If the object is equal to itself, we take the data of turns from it. If not equal, then disable
          (set `SpringArmComponent.SocketOffset` (`self.Body_offset`) _camera_arm)
          (if (== _target_lookat _target_follow)
            (`SceneComponent.K2_SetWorldRotation` _camera_arm (`KismetMathLibrary.ComposeRotators` (`SceneComponent.K2_GetComponentRotation` (`Actor.RootComponent` _target_follow)) (`self.Body_rotation_offset`)) false false)))))
    (:`then_2`
      ;[1 1 1] Follow_GetAllTransform
      (`/Engine/EditorBlueprintResources/StandardMacros.IsValid` (`self.Target_All_Transfrom`)
        (:`Is Valid`
          (`self.Follow_GetAllTransform`))))
    (:`then_3`
      ;[1 1 1] Camera Target in Zone
      (if (`self.TargetInZone?`)
        (bind _asstatic_mesh_actor (cast `StaticMeshActor` (stale `self.Sphere_radius_activated.OnComponentBeginOverlap` OtherActor) :!label _label))
        (set `self.Target_LookAT` _asstatic_mesh_actor)))
    (:`then_4`
      ;[0.4969 1 0.7305] System Screenshot (manual mode. Record when starting the game). Please check value  ScreenShot_Rec  - Must be switched-on. Update 1.13
      (if (`self.Rec`)
        (`/Engine/EditorBlueprintResources/StandardMacros.Do N` 1 :!label _label_2
          (:`Exit`
            (`GameplayStatics.SetGamePaused` true)
            (`self.StartScreenShot`)
            (`KismetSystemLibrary.Delay` (`self.DelayNextFrame`))
            (`GameplayStatics.SetGamePaused` false)
            (goto _label_2 :!via `Reset`)))))
    (:`then_5`
      ;[0.4969 1 0.7305] Off Rec if CurrentShot >= NumberOfFrames. Update 1.13
      (if (`self.Show number frame?`)
        (`KismetSystemLibrary.PrintString` (`KismetStringLibrary.Conv_DoubleToString` _current_shot) true true (struct :`R` 1.0 :`A` 1.0) 0.001))
      (if (>= _current_shot (`KismetMathLibrary.Conv_IntToDouble` (`self.Number of frames`)))
        (set `self.Rec` false)))
    (:`then_6`
      ;[0.9833 1 0.2681] Camera 2D stereo. Get settings from CinemaCam
      (bind _ascine_camera_actor (cast `CineCameraActor` (`self.Target_All_Transfrom`)))
      (bind _returnvalue (`CineCameraActor.GetCineCameraComponent` _ascine_camera_actor))
      (set `CineCameraComponent.Filmback` (`CineCameraComponent.Filmback` _returnvalue) _cinecamera2d)
      (set `CineCameraComponent.FocusSettings` (`CineCameraComponent.FocusSettings` _returnvalue) _cinecamera2d)
      (set `CineCameraComponent.LensSettings` (`CineCameraComponent.LensSettings` _returnvalue) _cinecamera2d)
      (set `CameraComponent.PostProcessSettings` (`CameraComponent.PostProcessSettings` _returnvalue) _cinecamera2d)
      (set `CineCameraComponent.CurrentFocalLength` (`CineCameraComponent.CurrentFocalLength` _returnvalue) _cinecamera2d)
      (set `CineCameraComponent.CurrentAperture` (`CineCameraComponent.CurrentAperture` _returnvalue) _cinecamera2d))))

(event `MovingCamera`
  (bind _movecamera (`self.MoveCamera`))
  (bind _spline (`/Game/Camera_360/Blueprints/Spline_for_Camera.Spline` (`self.SplineActor`)))
  (bind _returnvalue (`KismetMathLibrary.Lerp` 0.0 (`SplineComponent.GetSplineLength` _spline) (`self.Alpha`)))
  ;[1 1 1] Spline System. Spline camera movement
  (`TimelineComponent.SetPlayRate` _movecamera (* 0.01 (`self.Speed`)))
  (`TimelineComponent.SetNewTime` _movecamera (`self.StartOffset`))
  (bind (_direction _alpha) (`Timeline|MoveCamera`)
    (:`Update`
      (set `self.Alpha` _alpha)
      (`self.K2_SetActorLocationAndRotation` (`SplineComponent.GetLocationAtDistanceAlongSpline` _spline _returnvalue "World") (`SplineComponent.GetRotationAtDistanceAlongSpline` _spline _returnvalue "World")))
    (:`Finished`
      ;[1 1 1] Loop Path
      (`/Engine/EditorBlueprintResources/StandardMacros.IsValid` (`self.SplineActor`)
        (:`Is Valid`
          (if (`self.Closed_Loop?`)
            (`self.MovingCamera`)))))))

(event `self.Sphere_radius_activated.OnComponentBeginOverlap`
  (params (OverlappedComponent :type "PrimitiveComponent Object Reference") (OtherActor :type "Actor Object Reference") (OtherComp :type "PrimitiveComponent Object Reference") (OtherBodyIndex :type Integer) (bFromSweep :type Boolean) (SweepResult :type "HitResult Structure (by ref)"))
  ;[1 1 1] Camera Target in Zone
  (if (`self.Activate_Target_Zone?`)
    (set `self.TargetInZone?` true)
    (goto _label)))

(event `self.Sphere_radius_activated.OnComponentEndOverlap`
  (params (OverlappedComponent :type "PrimitiveComponent Object Reference") (OtherActor :type "Actor Object Reference") (OtherComp :type "PrimitiveComponent Object Reference") (OtherBodyIndex :type Integer))
  ;[1 1 1] Camera Target in Zone
  (if (`self.Activate_Target_Zone?`)
    (set `self.TargetInZone?` false)
    (set `self.Target_LookAT` null)
    (`SceneComponent.K2_SetWorldRotation` (`self.Camera_arm`) (`KismetMathLibrary.ComposeRotators` (`KismetMathLibrary.ComposeRotators` (`self.Camera_rotation_offset`) (`SceneComponent.K2_GetComponentRotation` (`self.Arrow_actor`))) (`self.Body_rotation_offset`)) false false)))

(event `StartScreenShot`
  ;[1 0.676 1] ScreenShot (If you need to restore the default path to save screenshots. Specify the / sign and the files will be saved to the standard folder.  Saved/Screenshots/Windows   )  Update 1.12
  (bind _output_get (set `self.NumberImage_manual` (+ (`self.NumberImage_manual`) 1) :!label _label_3))
  (`KismetSystemLibrary.ExecuteConsoleCommand` (`KismetStringLibrary.Replace` (`KismetStringLibrary.Concat_StrStr` "HighResShot " (`KismetStringLibrary.Conv_DoubleToString` (`self.Screenshot_Size_X`)) "x" (`KismetStringLibrary.Conv_DoubleToString` (`self.Screenshot_Size_Y`)) " " "filename=" (`self.Path`) "/" (`self.NameImage`) "_" (`KismetTextLibrary.Conv_TextToString` (`KismetTextLibrary.Conv_IntToText` _output_get false false 5)) ".png") "\\" "/") (`GameplayStatics.GetPlayerController` 0))
  (set `self.Current Shot` (+ (`self.Current Shot`) 1.0)))

(event `Key|M` :paused true
  (params (Key :type "Key Structure"))
  ;[1 0.676 1] ScreenShot (If you need to restore the default path to save screenshots. Specify the / sign and the files will be saved to the standard folder.  Saved/Screenshots/Windows   )  Update 1.12
  (:`Pressed`
    (goto _label_3)))

(event `Key|K` :paused true
  (params (Key :type "Key Structure"))
  ;[0.3813 1 0.1441] Debug Next Frame
  (:`Pressed`
    (`KismetSystemLibrary.Delay` (`self.DelayNextFrame`))
    (`GameplayStatics.SetGamePaused` true)
    (`self.StartScreenShot`)
    (`GameplayStatics.SetGamePaused` false)
    (`KismetSystemLibrary.Delay` 4e-06)
    (`GameplayStatics.SetGamePaused` true)))

(fn `Activation_Stereo2D`
  (bind _x (.x (`SceneComponent.RelativeLocation` (`self.CineCamera2D`))))
  ;[1 1 1] Right Eye and all properties for transform target
  (bind _returnvalue (`GameplayStatics.CreatePlayer` 0))
  (bind _returnvalue_2 (`|SpawnActorFromClass` "/Game/Camera_360/Blueprints/Camera2D_R.Camera2D_R_C" (`self.GetTransform`) "Undefined" "OverrideRootScale" _returnvalue null))
  (set `/Game/Camera_360/Blueprints/Camera2D_R.Target_All_Transfrom` (`self.Target_All_Transfrom`) _returnvalue_2)
  (set `/Game/Camera_360/Blueprints/Camera2D_R.Target_Follow` (`self.Target_Follow`) _returnvalue_2)
  (set `/Game/Camera_360/Blueprints/Camera2D_R.Target_LookAT` (`self.Target_LookAT`) _returnvalue_2)
  (set `/Game/Camera_360/Blueprints/Camera2D_R.Body_rotation_offset` (`self.Body_rotation_offset`) _returnvalue_2)
  (bind _output_get (set `/Game/Camera_360/Blueprints/Camera2D_R.Body_offset` (`self.Body_offset`) _returnvalue_2))
  (set `SpringArmComponent.SocketOffset` _output_get (`/Game/Camera_360/Blueprints/Camera2D_R.Camera_arm` _returnvalue_2))
  (set `SpringArmComponent.SocketOffset` (`self.Cam_Location_Offset `) (`/Game/Camera_360/Blueprints/Camera2D_R.Camera_Offset` _returnvalue_2))
  (bind _camera_offset (`/Game/Camera_360/Blueprints/Camera2D_R.Camera_Offset` _returnvalue_2))
  (`SceneComponent.K2_SetRelativeRotation` _camera_offset (`KismetMathLibrary.ComposeRotators` (`SceneComponent.RelativeRotation` _camera_offset) (`self.Cam_Rotation_Offset `)) false false)
  ;[1 1 1] Left Eye
  (bind _returnvalue_3 (`GameplayStatics.CreatePlayer` -1))
  (`PlayerController.SetViewTargetWithBlend` _returnvalue_3 self 0.0 "VTBlend_Linear" 0.0 false)
  ;[1 1 1] Right IPD
  (`SceneComponent.K2_SetRelativeLocation` (`self.CineCamera2D`) (`KismetMathLibrary.MakeVector` _x (+ _x (`self.IPD`)) (.z (`SceneComponent.RelativeLocation` (`self.CineCamera2D`)))) false false))

(fn `Apply max FPS for Editor`
  (`KismetSystemLibrary.ExecuteConsoleCommand` (`KismetStringLibrary.Concat_StrStr` "t.MaxFPS " (`KismetStringLibrary.Conv_DoubleToString` (`self.Max FPS for Editor`))) null))

(fn `Follow`
  (bind _target_follow (`self.Target_Follow`))
  ;[1 1 1] Camera point location to Target location and rotation(Working in Play mode).
  (`/Engine/EditorBlueprintResources/StandardMacros.IsValid` _target_follow
    (:`Is Valid`
      (`self.K2_SetActorLocation` (`SceneComponent.K2_GetComponentLocation` (`Actor.RootComponent` _target_follow))))))

(fn `Follow_GetAllTransform`
  ;[1 1 1] Get location and rotation from Target to Point Camera (Working in Play mode).
  (`SceneComponent.K2_SetWorldTransform` (`self.Root_Camera`) (`KismetMathLibrary.MakeTransform` (.location (`self.GetTransform` (`self.Target_All_Transfrom`))) (.rotation (`self.GetTransform` (`self.Target_All_Transfrom`)))) false false))

(fn `LookAT`
  ;[1 1 1] Find Target
  (`SceneComponent.K2_SetWorldRotation` (`self.Camera_arm`) (`KismetMathLibrary.ComposeRotators` (`KismetMathLibrary.FindLookAtRotation` (`self.K2_GetActorLocation`) (`SceneComponent.K2_GetComponentLocation` (`Actor.RootComponent` (`self.Target_LookAT`)))) (`self.Body_rotation_offset`)) false false))

(fn `UserConstructionScript`
  (bind _hidden_collision__arrow_ (`self.Hidden Collision, Arrow?`))
  (bind _scale_zone (`self.Scale_Zone`))
  (bind _splineactor (`self.SplineActor`))
  (bind _target_lookat (`self.Target_LookAT`))
  (bind _target_follow (`self.Target_Follow`))
  (bind _camera_arm (`self.Camera_arm`))
  (bind _target_all_transfrom (`self.Target_All_Transfrom`))
  (bind _camera_arm_2 (`self.Camera_arm`))
  (bind _camera_smooth_ (`self.Camera_Smooth?`))
  (bind _screenshot_size_x (`self.Screenshot_Size_X`))
  (bind _camera_offset (`self.Camera_Offset`))
  (bind _returnvalue (`SceneComponent.K2_GetComponentLocation` (`self.Camera_arm`)))
  (bind _returnvalue_2 (`KismetMathLibrary.ComposeRotators` (`KismetMathLibrary.ComposeRotators` (`self.Camera_rotation_offset`) (`self.K2_GetActorRotation`)) (`self.Body_rotation_offset`)))
  (bind _returnvalue_3 (`SceneComponent.K2_GetComponentLocation` (`Actor.RootComponent` _target_lookat)))
  (`|ExecutionSequence`
    (:`then_0`
      ;[1 1 1] Body. Camera point location to Target location and rotation(Working in Construction mode, and play).
      (set `SpringArmComponent.SocketOffset` (`self.Body_offset`) (`self.Camera_arm`))
      (`/Engine/EditorBlueprintResources/StandardMacros.IsValid` _target_follow
        (:`Is Valid`
          (`self.K2_SetActorLocation` (`SceneComponent.K2_GetComponentLocation` (`Actor.RootComponent` _target_follow)))
          (`self.K2_SetActorRotation` _returnvalue_2))
        (:`Is Not Valid`
          ;[1 1 1] Rotation for Spline
          (`SceneComponent.K2_SetWorldRotation` (`self.Camera_arm`) _returnvalue_2 false false :!label _label))))
    (:`then_1`
      ;[1 1 1] Find Target. Camera rotation, find Target location(Working in Construction mode and play).
      (`/Engine/EditorBlueprintResources/StandardMacros.IsValid` _target_lookat
        (:`Is Valid`
          (if (== (`self.Target_Follow`) (`self.Target_LookAT`))
            (`SceneComponent.K2_SetWorldRotation` _camera_arm_2 (`KismetMathLibrary.ComposeRotators` (`KismetMathLibrary.FindLookAtRotation` _returnvalue _returnvalue_3) (`self.Body_rotation_offset`)) false false)
            (else
              (`SceneComponent.K2_SetWorldRotation` _camera_arm_2 (`KismetMathLibrary.ComposeRotators` (`KismetMathLibrary.FindLookAtRotation` _returnvalue _returnvalue_3) (`self.Body_rotation_offset`)) false false))))
        (:`Is Not Valid`
          (goto _label))))
    (:`then_2`
      ;[1 1 1] camera smooth
      (set `SpringArmComponent.bUsePawnControlRotation` _camera_smooth_ _camera_arm)
      (set `SpringArmComponent.bEnableCameraRotationLag` _camera_smooth_ _camera_arm)
      (set `SpringArmComponent.CameraRotationLagSpeed` (`self.Smooth_Camera`) _camera_arm))
    (:`then_3`
      ;[1 1 1] Spline. Closed loop>?
      (`/Engine/EditorBlueprintResources/StandardMacros.IsValid` _splineactor
        (:`Is Valid`
          (`SplineComponent.SetClosedLoop` (`/Game/Camera_360/Blueprints/Spline_for_Camera.Spline` _splineactor) (`self.Closed_Loop?`) true))))
    (:`then_4`
      ;[1 1 1] Zone Activation Cam to target
      (`SceneComponent.SetWorldScale3D` (`self.Sphere_radius_activated`) (`KismetMathLibrary.MakeVector` _scale_zone _scale_zone _scale_zone))
      ;[1 1 1] Hidden collision zone or arrow?
      (`SceneComponent.SetHiddenInGame` (`self.Sphere_radius_activated`) _hidden_collision__arrow_ false)
      (`SceneComponent.SetHiddenInGame` (`self.Arrow_camera`) _hidden_collision__arrow_ false)
      (`SceneComponent.SetHiddenInGame` (`self.Arrow_actor`) _hidden_collision__arrow_ false)
      (if _hidden_collision__arrow_
        (`SceneComponent.SetVisibility` (`self.Sphere_radius_activated`) false false)
        (`SceneComponent.SetVisibility` (`self.Arrow_camera`) false false)
        (`SceneComponent.SetVisibility` (`self.Arrow_actor`) false false)))
    (:`then_5`
      ;[1 1 1] Follow_GetAllTransform from Target
      (`/Engine/EditorBlueprintResources/StandardMacros.IsValid` _target_all_transfrom
        (:`Is Valid`
          (`SceneComponent.K2_SetWorldTransform` (`self.Root_Camera`) (`KismetMathLibrary.MakeTransform` (.location (`self.GetTransform` _target_all_transfrom)) (.rotation (`self.GetTransform` _target_all_transfrom))) false false))))
    (:`then_6`
      ;[0.4702 1 0.01995] Loc and Rot Offset Camera2D Update 1.13 fix
      (set `SpringArmComponent.SocketOffset` (`self.Cam_Location_Offset `) (`self.Camera_Offset`))
      (`SceneComponent.K2_SetRelativeRotation` _camera_offset (`KismetMathLibrary.ComposeRotators` (`SceneComponent.RelativeRotation` _camera_offset) (`self.Cam_Rotation_Offset `)) false false))
    (:`then_7`
      ;[0.5428 1 0.1453] Aspect Ratioo 16:9 for ScreenShot Size. Update 1.13 fix
      (if (`self.Size 16:9?`)
        (set `self.Screenshot_Size_Y` (/ _screenshot_size_x 1.777777778))
        (else
          (set `self.Screenshot_Size_X` _screenshot_size_x)
          (set `self.Screenshot_Size_Y` (`self.Screenshot_Size_Y`)))))))