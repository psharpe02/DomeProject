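; Camera_Rec_2D is a capture Blueprint that saves numbered screenshots for the 360 camera tool.
; Each StartScreenShot_camera_360 call switches to unlit view, increments the image counter and runs a HighResShot console command.
; That command is built from the configured resolution, path and name, with a five-digit PNG suffix and forward slashes.
; EndPlay issues a console command resetting the force-all ray tracing effects setting to -1.
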(event `self.ReceiveEndPlay`
  (params (EndPlayReason :type "EEndPlayReason Enum" :default "Destroyed"))
  ;[1 1 1] Raytracing On
  (`KismetSystemLibrary.ExecuteConsoleCommand` "r.raytracing.ForceAllRayTracingEffects -1" null))

(event `StartScreenShot_camera_360`
  ;[1 0.4681 0.07743] Image 360 screenshot
  (`KismetSystemLibrary.ExecuteConsoleCommand` "viewmode unlit" null)
  (bind _output_get (set `self.NumberImage_360` (+ (`self.NumberImage_360`) 1)))
  (`KismetSystemLibrary.ExecuteConsoleCommand` (`KismetStringLibrary.Replace` (`KismetStringLibrary.Concat_StrStr` "HighResShot " (`KismetStringLibrary.Conv_DoubleToString` (`self.Screenshot_Size360_X`)) "x" (`KismetStringLibrary.Conv_DoubleToString` (`self.Screenshot_Size360_Y`)) " " "filename=" (`self.PathImage360`) "/" (`self.NameImage360`) "_" (`KismetTextLibrary.Conv_TextToString` (`KismetTextLibrary.Conv_IntToText` _output_get false false 5)) ".png") "\\" "/") (`GameplayStatics.GetPlayerController` 0)))

(fn `UserConstructionScript`)