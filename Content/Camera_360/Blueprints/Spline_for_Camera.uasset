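; Spline actor for the 360 camera system that places a visible, numbered marker at each point of its spline.
; The construction script adds a Point_for_spline child actor component at every point's local location, rotates it to match the spline and sets its text to the point index.
; The spawned markers are stored in the Child array, and the event graph holds no runtime logic.
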(fn `UserConstructionScript`
  (bind _spline (`self.Spline`))
  (bind _index (`self.Index`))
  ;[1 1 1] Spline System
  (bind _output_get (set `self.Number of spline points` (- (`SplineComponent.GetNumberOfSplinePoints` (`self.Spline`)) 1)))
  (for _index_2 (range (+ _output_get 1))
    (bind _output_get_2 (set `self.Index` _index_2))
    (bind _returnvalue (`AddComponent|NODE_AddChildActorComponent-1` :`RelativeTransform` (`KismetMathLibrary.Conv_VectorToTransform` (`SplineComponent.GetLocationAtSplinePoint` _spline _index "Local"))))
    (`ChildActorComponent.SetChildActorClass` _returnvalue "/Game/Camera_360/Blueprints/Point_for_spline.Point_for_spline_C")
    ;;[1 1 1] Cast to Point for Spline (models and text)
    (bind _aspoint_for_spline (cast `/Game/Camera_360/Blueprints/Point_for_spline` (`ChildActorComponent.ChildActor` _returnvalue)))
    (`KismetArrayLibrary.Array_Add` (`self.Child`) _aspoint_for_spline)
    (`TextRenderComponent.K2_SetText` (`/Game/Camera_360/Blueprints/Point_for_spline.TextRender` _aspoint_for_spline) (`KismetTextLibrary.Conv_IntToText` _output_get_2))
    (`SceneComponent.K2_SetRelativeRotation` (`Actor.RootComponent` _aspoint_for_spline) (`SplineComponent.GetRotationAtSplinePoint` _spline _index "Local") false false)))