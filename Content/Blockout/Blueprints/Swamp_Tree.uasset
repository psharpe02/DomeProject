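; Blockout swamp tree actor that can appear as either a full tree or a stump.
; The construction script reads TreeType and shows the matching SwampTree or SwampStump component while hiding the other, leaving both untouched for other values.
; The event graph holds only disabled default events, so there is no runtime behavior.
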(fn `UserConstructionScript`
  (bind _swamptree (`self.SwampTree`))
  (bind _swampstump (`self.SwampStump`))
  (if (== (`self.TreeType`) 1)
    (`SceneComponent.SetVisibility` _swamptree true false)
    (`SceneComponent.SetVisibility` _swampstump false false)
    (elif (== (`self.TreeType`) 2)
      (`SceneComponent.SetVisibility` _swampstump true false)
      (`SceneComponent.SetVisibility` _swamptree false false))))