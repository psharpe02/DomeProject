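; Forest_Tree is a blockout forest tree actor that can display one of two tree variants.
; The Construction Script reads TreeType and shows either the ForestTree1 or ForestTree2 component while hiding the other.
; Values other than the two handled types leave both components' visibility unchanged, and the event graph has no active logic.
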(fn `UserConstructionScript`
  (bind _forest_tree1 (`self.Forest_Tree1`))
  (bind _forest_tree2 (`self.Forest_Tree2`))
  (if (== (`self.TreeType`) 1)
    (`SceneComponent.SetVisibility` _forest_tree1 true false)
    (`SceneComponent.SetVisibility` _forest_tree2 false false)
    (elif (== (`self.TreeType`) 2)
      (`SceneComponent.SetVisibility` _forest_tree2 true false)
      (`SceneComponent.SetVisibility` _forest_tree1 false false))))